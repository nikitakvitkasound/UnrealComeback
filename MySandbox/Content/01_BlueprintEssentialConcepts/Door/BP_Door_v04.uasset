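; BP_Door_v04 is a swinging door that the player opens or closes with the E key while inside its trigger box.
; Entering the box prints a prompt, enables input, opens a gate and picks the swing direction from the player's side in door-local space.
; The DoorPivot timeline drives the mesh yaw, playing or reversing on E.
; Leaving the box disables input and reverses the timeline to close the door.
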(event OnComponentBeginOverlap(Box)
  (params (OverlappedComponent :type Primitive%20Component%20Object%20Reference) (OtherActor :type Actor%20Object%20Reference) (OtherComp :type Primitive%20Component%20Object%20Reference) (OtherBodyIndex :type Integer) (bFromSweep :type Boolean) (SweepResult :type Hit%20Result%20Structure%20%28by%20ref%29))
  (bind _returnvalue (Game|Player|GetPlayerPawn 0))
  (if (== OtherActor _returnvalue)
    (Variables|Default|SetDoorOpenDirection (> (.X (Math|Vector|BreakVector (Math|Vector|UnrotateVector (- (Transformation|GetActorLocation) (Transformation|GetActorLocation _returnvalue)) (Transformation|GetActorRotation)))) 0.0))
    (Development|PrintString "PRESS ' E' TO OPEN OR CLOSE THE DOOR" true true "(R=0.000000,G=0.660000,B=1.000000,A=1.000000)" 6.0)
    (Input|EnableInput (Game|GetPlayerController 0))
    (Utilities|FlowControl|Gate true) ; enters at Open
  ))

(event OnComponentEndOverlap(Box)
  (params (OverlappedComponent :type Primitive%20Component%20Object%20Reference) (OtherActor :type Actor%20Object%20Reference) (OtherComp :type Primitive%20Component%20Object%20Reference) (OtherBodyIndex :type Integer))
  (if (== (Game|Player|GetPlayerPawn 0) OtherActor)
    (Input|DisableInput (Game|GetPlayerController 0))
    (bind _yaw (Timeline|Door%20Pivot Reverse)
      (:Update
        (bind _output_get (Variables|Default|SetDoorYaw _yaw))
        (Transformation|SetRelativeRotation (Variables|Default|GetSM_Door) (Math|Rotator|MakeRotator 0.0 0.0 (* _output_get (Math|Float|SelectFloat 1.0 -1.0 (Variables|Default|GetDoorOpenDirection)))) false false)))))

(event Input|KeyboardEvents|E
  (params (Key :type Key%20Structure :default "None"))
  (:Pressed
    (if (> (Variables|Default|GetDoorYaw) 0.0)
      (bind _yaw (Timeline|Door%20Pivot Reverse)
        (:Update
          (bind _output_get (Variables|Default|SetDoorYaw _yaw))
          (Transformation|SetRelativeRotation (Variables|Default|GetSM_Door) (Math|Rotator|MakeRotator 0.0 0.0 (* _output_get (Math|Float|SelectFloat 1.0 -1.0 (Variables|Default|GetDoorOpenDirection)))) false false)))
      (else
        (Utilities|FlowControl|Gate true
          (:Exit
            (Timeline|Door%20Pivot Play)))))))

(fn ConstructionScript)