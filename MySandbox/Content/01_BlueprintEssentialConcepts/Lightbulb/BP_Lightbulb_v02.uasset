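; BP_Lightbulb_v02 is a proximity-triggered lightbulb that turns on in a random color when the player walks near it.
; The light starts dark at BeginPlay.
; When the player pawn enters the Box trigger, LightSource gets a randomized RGB color and full intensity, and leaving the box switches it off again.
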(event OnComponentBeginOverlap(Box)
  (params (OverlappedComponent :type Primitive%20Component%20Object%20Reference) (OtherActor :type Actor%20Object%20Reference) (OtherComp :type Primitive%20Component%20Object%20Reference) (OtherBodyIndex :type Integer) (bFromSweep :type Boolean) (SweepResult :type Hit%20Result%20Structure%20%28by%20ref%29))
  (bind _lightsource (Variables|Default|GetLightSource))
  (if (== OtherActor (Game|Player|GetPlayerPawn 0))
    (Rendering|Components|Light|SetLightColor _lightsource (Utilities|Struct|MakeLinearColor (Math|Random|RandomFloat) (Math|Random|RandomFloat) (Math|Random|RandomFloat) 1.0) true)
    (Rendering|Components|Light|SetIntensity _lightsource 5e+03)))

(event OnComponentEndOverlap(Box)
  (params (OverlappedComponent :type Primitive%20Component%20Object%20Reference) (OtherActor :type Actor%20Object%20Reference) (OtherComp :type Primitive%20Component%20Object%20Reference) (OtherBodyIndex :type Integer))
  (if (== (Game|Player|GetPlayerPawn 0) OtherActor)
    (Rendering|Components|Light|SetIntensity (Variables|Default|GetLightSource) 0.0)))

(event EventBeginPlay
  (Rendering|Components|Light|SetIntensity (Variables|Default|GetLightSource) 0.0))

(fn ConstructionScript)