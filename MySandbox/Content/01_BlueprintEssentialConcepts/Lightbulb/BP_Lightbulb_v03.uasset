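; BP_Lightbulb is a wall lamp whose light brightens as the player pawn approaches it.
; Entering the Box trigger records the pawn's horizontal distance and starts a fast looping timer that remaps the current distance to light intensity, unclamped.
; Leaving the box clears the timer and turns the light off, its initial state.
; The lamp's hit event reaches a DoOnce with no visible effect.
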(event OnComponentBeginOverlap(Box)
  (params (OverlappedComponent :type Primitive%20Component%20Object%20Reference) (OtherActor :type Actor%20Object%20Reference) (OtherComp :type Primitive%20Component%20Object%20Reference) (OtherBodyIndex :type Integer) (bFromSweep :type Boolean) (SweepResult :type Hit%20Result%20Structure%20%28by%20ref%29))
  (if (== OtherActor (Game|Player|GetPlayerPawn 0))
    (bind _returnvalue (Utilities|Time|SetTimerbyEvent (delegate Custom|GetDistanceBetweenTwoActors) 0.01 true))
    (Variables|Default|SetTimerHandle _returnvalue)
    (bind _output_get (Variables|Default|SetMaxDistanceToActor (Transformation|GetHorizontalDistanceTo (Game|Player|GetPlayerPawn 0))))))

(event OnComponentEndOverlap(Box)
  (params (OverlappedComponent :type Primitive%20Component%20Object%20Reference) (OtherActor :type Actor%20Object%20Reference) (OtherComp :type Primitive%20Component%20Object%20Reference) (OtherBodyIndex :type Integer))
  (if (== (Game|Player|GetPlayerPawn 0) OtherActor)
    (Utilities|Time|ClearandInvalidateTimerbyHandle (Variables|Default|GetTimerHandle))
    (Rendering|Components|Light|SetIntensity (Variables|Default|GetLightSource) 0.0)))

(event OnComponentHit(LampWall)
  (params (HitComponent :type Primitive%20Component%20Object%20Reference) (OtherActor :type Actor%20Object%20Reference) (OtherComp :type Primitive%20Component%20Object%20Reference) (NormalImpulse :type Vector :default "0, 0, 0") (Hit :type Hit%20Result%20Structure%20%28by%20ref%29))
  (Utilities|FlowControl|DoOnce false))

(event Custom|GetDistanceBetweenTwoActors
  (Rendering|Components|Light|SetIntensity (Variables|Default|GetLightSource) (Math|Float|MapRangeUnclamped (Transformation|GetHorizontalDistanceTo (Game|Player|GetPlayerPawn 0)) (stale OnComponentBeginOverlap(Box) _output_get) 7e+01 0.0 5e+03)))

(event EventBeginPlay
  (Rendering|Components|Light|SetIntensity (Variables|Default|GetLightSource) 0.0))

(fn ConstructionScript)