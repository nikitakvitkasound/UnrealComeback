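; Spotlight actor that sweeps back and forth until its beam trace detects an object, then turns toward the player.
; A Patrol timeline yaws the hinge, with a FlipFlop alternating play and reverse.
; Every Tick, a debug-drawn multi-object line trace runs along the body's forward vector.
; A hit stops the patrol and splits the look-at rotation into body pitch and hinge yaw; a miss only prints the result.
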(event Custom|Start%20Patrol
  (Utilities|FlowControl|FlipFlop
    (:A
      (bind _turn_90 (Timeline|Patrol Play)
        (:Update
          (Transformation|SetRelativeRotation (Variables|Default|GetSpotlightHinge) (Math|Rotator|MakeRotator 0.0 0.0 _turn_90) false false))
        (:Finished
          (CallFunction|StartPatrol))))
    (:B
      (Timeline|Patrol Reverse))))

(event Custom|Stop%20Patrol
  (bind _turn_90 (Timeline|Patrol Stop)
    (:Update
      (Transformation|SetRelativeRotation (Variables|Default|GetSpotlightHinge) (Math|Rotator|MakeRotator 0.0 0.0 _turn_90) false false))
    (:Finished
      (CallFunction|StartPatrol))))

(event EventTick
  (params (DeltaSeconds :type Float%20%28single-precision%29))
  (bind _returnvalue (Game|Player|GetPlayerPawn 0))
  (bind _returnvalue_2 (Transformation|GetActorLocation))
  (bind _spotlightbody (Variables|Default|GetSpotlightBody))
  (bind _returnvalue_3 (Transformation|GetWorldLocation _spotlightbody))
  (bind _returnvalue_4 (Transformation|GetActorLocation _returnvalue))
  (bind _returnvalue_5 (Math|Rotator|FindLookatRotation _returnvalue_2 _returnvalue_4))
  (bind (_roll _pitch _yaw) (Math|Rotator|BreakRotator _returnvalue_5))
  (bind _returnvalue_6 (Class|KismetSystemLibrary|LineTraceMultiforObjects _returnvalue_3 (+ _returnvalue_3 (* (Math|Vector|GetForwardVector (Transformation|GetWorldRotation _spotlightbody)) (Variables|Default|GetLinetraceScale))) (Variables|Default|GetObject%20Types) false 0 "ForOneFrame" true))
  (if _returnvalue_6
    (CallFunction|StopPatrol)
    (Transformation|SetRelativeRotation (Variables|Default|GetSpotlightBody) (Math|Rotator|MakeRotator 0.0 _pitch 0.0) false false)
    (Transformation|SetRelativeRotation (Variables|Default|GetSpotlightHinge) (Math|Rotator|MakeRotator 0.0 0.0 _yaw) false false)
    (else
      (Development|PrintString (Utilities|String|ToString(Boolean) _returnvalue_6)))))

(event EventBeginPlay
  (Transformation|SetRelativeRotation (Variables|Default|GetSpotlightBody) "-40.000000,0.000000,0.000000" false false)
  (CallFunction|StartPatrol))

(fn ConstructionScript)